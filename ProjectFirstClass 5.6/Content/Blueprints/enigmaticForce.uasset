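; Rising force actor whose Cube climbs toward the height read from the Flicker actor.
; Each Tick, a tick-counting timer steps up the climb speed at two thresholds and moves the Cube upward.
; Nearing that height zeroes the speed and stops the timer for good; a Flicker overlapping the Box also zeroes speed after a delay.
; Spin and bubble-spawning helper functions are defined but not called here.
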(event `self.ReceiveBeginPlay`
  (set `self.canMove` true))

(event `self.ReceiveTick`
  (params (DeltaSeconds :type "Float (single-precision)"))
  (bind _cube (`self.Cube`))
  (bind (_returnvalue_x _returnvalue_y _returnvalue_z) (`KismetMathLibrary.BreakVector` (`SceneComponent.K2_GetComponentLocation` _cube)))
  (bind (_relativelocation_x _relativelocation_y _relativelocation_z) (`KismetMathLibrary.BreakVector` (`SceneComponent.RelativeLocation` _cube)))
  (bind _returnvalue (`GameplayStatics.GetActorOfClass` "/Game/FlickerBPs/Blueprints/Flicker.Flicker_C"))
  (`/Engine/EditorBlueprintResources/StandardMacros.IsValid` _returnvalue
    (:`Is Valid`
      (set `self.heightEquiv` (`/Game/FlickerBPs/Blueprints/Flicker.playerHeight` _returnvalue)))
    (:`Is Not Valid`
      _))
  (set `self.zPos` (/ (- _returnvalue_z 178.34491) 10.0))
  (if (>= (`self.zPos`) (- (`self.heightEquiv`) 50.0))
    (set `self.canCountUp` false)
    (set `self.upSpeed` 0.0)
    (else
      (`self.timeSpeedManager`)
      (`KismetSystemLibrary.MoveComponentTo` _cube (`KismetMathLibrary.MakeVector` _relativelocation_x _relativelocation_y (+ _relativelocation_z (`self.upSpeed`)))))))

(event `self.Box.OnComponentBeginOverlap`
  (params (OverlappedComponent :type "PrimitiveComponent Object Reference") (OtherActor :type "Actor Object Reference") (OtherComp :type "PrimitiveComponent Object Reference") (OtherBodyIndex :type Integer) (bFromSweep :type Boolean) (SweepResult :type "HitResult Structure (by ref)"))
  (cast `/Game/FlickerBPs/Blueprints/Flicker` OtherActor)
  (`KismetSystemLibrary.Delay` 1.0)
  (set `self.upSpeed` 0.0))

(fn `spawnBubbles`
  (params (spawnPt :type "ArrowComponent Object Reference"))
  (bind _returnvalue_location (`KismetMathLibrary.BreakTransform` (`SceneComponent.K2_GetComponentToWorld` spawnPt)))
  (bind _spawncountdown (`self.spawnCountDown`))
  (set `self.spawnCountDown` (- _spawncountdown 1.0))
  (if (<= _spawncountdown 0.0)
    (`|SpawnActorFromClass` "/Game/Blueprints/force_bubbleParticle_BP.force_bubbleParticle_BP_C" (`KismetMathLibrary.MakeTransform` _returnvalue_location) "Undefined" "MultiplyWithRoot" null null)
    (set `self.spawnCountDown` (`self.spawnTImeStart`))))

(fn `spin`
  (bind _cube (`self.Cube`))
  (bind _returnvalue (`SceneComponent.GetRelativeTransform` _cube))
  (`SceneComponent.K2_SetRelativeRotation` _cube (`KismetMathLibrary.MakeRotator` (.roll (.rotation _returnvalue)) (.pitch (.rotation _returnvalue)) (+ (.yaw (.rotation _returnvalue)) (`self.rotatingSpeed`))) false false))

(fn `timeSpeedManager`
  (bind _timer (`self.timer`))
  (if (`self.canCountUp`)
    (set `self.timer` (+ _timer 1.0))
    (if (and (>= _timer 2000.0) (< _timer 4500.0))
      (set `self.upSpeed` 35.0)
      (elif (>= _timer 4500.0)
        (set `self.upSpeed` 53.0)))))

(fn `UserConstructionScript`)