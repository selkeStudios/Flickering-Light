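; Trunk_BP is a self-chaining level segment that fills itself with random ledges and obstacles.
; BeginPlay shuffles an integer array to choose four piece types, each spawned around a pair of markers with random X offset.
; The first trunk immediately spawns its successor; others do once Flicker overlaps either box, setting PrevRandom afterwards, intended to avoid repeats.
; A trunk destroys itself when enigMaticForce leaves its first box.
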(event `self.ReceiveBeginPlay`
  (bind _randomintarray (`self.randomIntArray`))
  (bind _output (`|GetArrayItem` _randomintarray))
  (bind _output_2 (`|GetArrayItem` _randomintarray 3))
  (`KismetArrayLibrary.Array_Shuffle` _randomintarray)
  (if (== _output (`self.prevRandom`))
    (`KismetArrayLibrary.Array_Remove` _randomintarray _output))
  (`self.spawnRandomLedges` (`self.obstaclePos`) (`self.obstaclePos1`) _output)
  (`self.spawnRandomLedges` (`self.obstaclePos2`) (`self.obstaclePos3`) (`|GetArrayItem` _randomintarray 1))
  (`self.spawnRandomLedges` (`self.obstaclePos4`) (`self.obstaclePos5`) (`|GetArrayItem` _randomintarray 2))
  (`self.spawnRandomLedges` (`self.obstaclePos6`) (`self.obstaclePos7`) _output_2)
  (if (`self.isFirstTrunk`)
    (if (not (`self.hasSpawnedNext`))
      (bind _returnvalue (`|SpawnActorFromClass` "trunk_BP_C" (`SceneComponent.K2_GetComponentToWorld` (`self.spawnNextTrunk`)) "Undefined" "OverrideRootScale" null null))
      (set `self.hasSpawnedNext` true)
      (set `/Game/Blueprints/trunk_BP.prevRandom` _output_2 _returnvalue))))

(event `self.Box.OnComponentBeginOverlap`
  (params (OverlappedComponent :type "PrimitiveComponent Object Reference") (OtherActor :type "Actor Object Reference") (OtherComp :type "PrimitiveComponent Object Reference") (OtherBodyIndex :type Integer) (bFromSweep :type Boolean) (SweepResult :type "HitResult Structure (by ref)"))
  (if (not (`self.hasSpawnedNext`))
    (cast `/Game/FlickerBPs/Blueprints/Flicker` OtherActor)
    (bind _returnvalue (`|SpawnActorFromClass` "trunk_BP_C" (`SceneComponent.K2_GetComponentToWorld` (`self.spawnNextTrunk`)) "Undefined" "OverrideRootScale" null null :!label _label))
    (set `self.hasSpawnedNext` true)
    (set `/Game/Blueprints/trunk_BP.prevRandom` (`|GetArrayItem` (`self.randomIntArray`) 3) _returnvalue)))

(event `self.Box1.OnComponentBeginOverlap`
  (params (OverlappedComponent :type "PrimitiveComponent Object Reference") (OtherActor :type "Actor Object Reference") (OtherComp :type "PrimitiveComponent Object Reference") (OtherBodyIndex :type Integer) (bFromSweep :type Boolean) (SweepResult :type "HitResult Structure (by ref)"))
  (if (not (`self.hasSpawnedNext`))
    (cast `/Game/FlickerBPs/Blueprints/Flicker` OtherActor)
    (goto _label)))

(event `self.Box.OnComponentEndOverlap`
  (params (OverlappedComponent :type "PrimitiveComponent Object Reference") (OtherActor :type "Actor Object Reference") (OtherComp :type "PrimitiveComponent Object Reference") (OtherBodyIndex :type Integer))
  (cast `/Game/Blueprints/enigmaticForce` OtherActor)
  (`self.K2_DestroyActor`))

(event `self.ReceiveTick`
  (params (DeltaSeconds :type "Float (single-precision)")))

(fn `randomZerotoFive`
  (returns (intThatIsRand :type Integer)))

(fn `spawnRandomLedges`
  (params (`[0]` :type "ArrowComponent Object Reference") (`[1]` :type "ArrowComponent Object Reference") (randomToSpawn :type Integer))
  (returns (RandomValue :type Integer))
  (bind (_returnvalue_x _returnvalue_y _returnvalue_z) (`KismetMathLibrary.BreakVector` (`SceneComponent.K2_GetComponentLocation` (`|GetArrayItem` (`|MakeArray` `[0]` `[1]`) (`KismetMathLibrary.RandomIntegerInRange` 0 1)))))
  (bind _returnvalue (+ (`KismetMathLibrary.RandomFloatInRange` -170.0 90.0) _returnvalue_x))
  (if (== randomToSpawn 0)
    (`|SpawnActorFromClass` "/Game/Blueprints/testLedge.testLedge_C" (`KismetMathLibrary.MakeTransform` (`KismetMathLibrary.MakeVector` _returnvalue _returnvalue_y _returnvalue_z)) "Undefined" "OverrideRootScale" null null)
    (return randomToSpawn)
    (elif (== randomToSpawn 1)
      (`|SpawnActorFromClass` "/Game/Blueprints/explodingLedge.explodingLedge_C" (`KismetMathLibrary.MakeTransform` (`KismetMathLibrary.MakeVector` _returnvalue _returnvalue_y _returnvalue_z)) "Undefined" "OverrideRootScale" null null)
      (return randomToSpawn)
      (elif (== randomToSpawn 2)
        (`|SpawnActorFromClass` "/Game/Blueprints/circleLedge.circleLedge_C" (`KismetMathLibrary.MakeTransform` (`KismetMathLibrary.MakeVector` _returnvalue _returnvalue_y _returnvalue_z)) "Undefined" "OverrideRootScale" null null)
        (return randomToSpawn)
        (elif (== randomToSpawn 3)
          (`|SpawnActorFromClass` "/Game/Blueprints/obstacle.obstacle_C" (`KismetMathLibrary.MakeTransform` (`KismetMathLibrary.MakeVector` _returnvalue _returnvalue_y _returnvalue_z)) "Undefined" "OverrideRootScale" null (200.0 0.0 0.0) (-200.0 0.0 0.0) null)
          (return randomToSpawn)
          (elif (== randomToSpawn 4)
            (`|SpawnActorFromClass` "/Game/Blueprints/movingLedge.movingLedge_C" (`KismetMathLibrary.MakeTransform` (`KismetMathLibrary.MakeVector` _returnvalue _returnvalue_y _returnvalue_z)) "Undefined" "OverrideRootScale" null null)
            (return randomToSpawn)
            (elif (== randomToSpawn 5)
              (`|SpawnActorFromClass` "/Game/Blueprints/orbitingLedge.orbitingLedge_C" (`KismetMathLibrary.MakeTransform` (`KismetMathLibrary.MakeVector` _returnvalue _returnvalue_y _returnvalue_z)) "Undefined" "OverrideRootScale" null null))))))))

(fn `UserConstructionScript`)