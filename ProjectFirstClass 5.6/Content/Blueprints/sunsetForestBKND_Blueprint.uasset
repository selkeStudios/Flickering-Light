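; Sunset forest background segment that chains copies of itself to form a continuing backdrop.
; The segment marked FirstImage spawns the next at its NextImageSpawn point on BeginPlay; others do so when a Flicker actor enters their Box.
; A HasSpawned flag limits each segment to one successor, spawned with a fixed 180-degree rotation.
; A segment destroys itself when an enigMaticForce actor leaves its Box.
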(event `self.ReceiveBeginPlay`
  (if (`self.firstImage`)
    (if (not (`self.hasSpawned`))
      (`|SpawnActorFromClass` "sunsetForestBKND_Blueprint_C" (`KismetMathLibrary.MakeTransform` (`SceneComponent.K2_GetComponentLocation` (`self.nextImageSpawn`)) (struct :`Yaw` 180.0)) "Undefined" "MultiplyWithRoot" null null)
      (set `self.hasSpawned` true))))

(event `self.Box.OnComponentBeginOverlap`
  (params (OverlappedComponent :type "PrimitiveComponent Object Reference") (OtherActor :type "Actor Object Reference") (OtherComp :type "PrimitiveComponent Object Reference") (OtherBodyIndex :type Integer) (bFromSweep :type Boolean) (SweepResult :type "HitResult Structure (by ref)"))
  (cast `/Game/FlickerBPs/Blueprints/Flicker` OtherActor)
  (if (not (`self.hasSpawned`))
    (`|SpawnActorFromClass` "sunsetForestBKND_Blueprint_C" (`KismetMathLibrary.MakeTransform` (`SceneComponent.K2_GetComponentLocation` (`self.nextImageSpawn`)) (struct :`Yaw` 180.0)) "Undefined" "MultiplyWithRoot" null null)
    (set `self.hasSpawned` true)))

(event `self.Box.OnComponentEndOverlap`
  (params (OverlappedComponent :type "PrimitiveComponent Object Reference") (OtherActor :type "Actor Object Reference") (OtherComp :type "PrimitiveComponent Object Reference") (OtherBodyIndex :type Integer))
  (cast `/Game/Blueprints/enigmaticForce` OtherActor)
  (`self.K2_DestroyActor`))

(fn `UserConstructionScript`)