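; A moving circular ledge that orbits its spawn point in the vertical XZ plane, in a random clockwise or counter-clockwise direction.
; Tick accumulates an angle and RotateOnY positions it on the radius around Y, while very low global time dilation zeroes its speed.
; Flicker overlap calls StopAndFlick on it and halts the orbit if Flicker is alive, resuming shortly after exit.
; Ending overlap with enigMaticForce destroys the ledge.
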(event `self.ReceiveActorEndOverlap`
  (params (OtherActor :type "Actor Object Reference"))
  (cast `/Game/Blueprints/enigMaticForce` OtherActor)
  (`self.K2_DestroyActor`))

(event `self.ReceiveBeginPlay`
  (set `self.initialLocation` (`self.K2_GetActorLocation`))
  (if (== (`KismetMathLibrary.RandomIntegerInRange` 0 1) 0)
    (set `self.isClockWise` true)
    (else
      (set `self.isClockWise` false))))

(event `self.ReceiveTick`
  (params (DeltaSeconds :type "Float (single-precision)"))
  (if (<= (`GameplayStatics.GetGlobalTimeDilation`) 0.2)
    (set `self.rotationSpeed` 0.0)
    (else
      (set `self.currentRot` (+ (`self.currentRot`) (* (* (`self.rotationSpeed`) DeltaSeconds) (`KismetMathLibrary.SelectFloat` 1.0 -1.0 (`self.isClockWise`)))))
      (`self.rotateOnY` self (`self.initialLocation`) (`self.radius`) (`self.startAngle`) (`self.currentRot`)))))

(event `self.Box.OnComponentBeginOverlap`
  (params (OverlappedComponent :type "PrimitiveComponent Object Reference") (OtherActor :type "Actor Object Reference") (OtherComp :type "PrimitiveComponent Object Reference") (OtherBodyIndex :type Integer) (bFromSweep :type Boolean) (SweepResult :type "HitResult Structure (by ref)"))
  (bind _asflicker (cast `/Game/FlickerBPs/Blueprints/Flicker` OtherActor))
  (`/Game/FlickerBPs/Blueprints/Flicker.stopAndFlick` _asflicker (`self.Cube`))
  (if (not (`/Game/FlickerBPs/Blueprints/Flicker.isDead` _asflicker))
    (set `self.rotationSpeed` 0.0)))

(event `self.Box.OnComponentEndOverlap`
  (params (OverlappedComponent :type "PrimitiveComponent Object Reference") (OtherActor :type "Actor Object Reference") (OtherComp :type "PrimitiveComponent Object Reference") (OtherBodyIndex :type Integer))
  (cast `/Game/FlickerBPs/Blueprints/Flicker` OtherActor)
  (`KismetSystemLibrary.Delay` 0.3)
  (set `self.rotationSpeed` 125.0))

(fn `rotateOnY`
  (params (actorToRotate :type "Actor Object Reference") (targetLocation :type "Vector Structure") (radius :type "Float (double-precision)") (angle :type "Float (double-precision)") (rotationRate :type "Float (double-precision)"))
  (returns (newPos :type "Vector Structure"))
  (locals (localActorToRotate :type "Actor Object Reference") (LocalLocation :type "Vector Structure") (Local_Radius :type "Float (double-precision)") (Local_Angle :type "Float (double-precision)") (Local_RotRate :type "Float (double-precision)"))
  (set `local.localActorToRotate` actorToRotate)
  (set `local.LocalLocation` targetLocation)
  (set `local.Local_Radius` radius)
  (set `local.Local_Angle` angle)
  (set `local.Local_RotRate` rotationRate)
  (`self.K2_SetActorLocation` (`local.localActorToRotate`) (+ (`local.LocalLocation`) (`KismetMathLibrary.RotateAngleAxis` (`KismetMathLibrary.MakeVector` (`local.Local_Radius`)) (+ (`local.Local_RotRate`) (`local.Local_Angle`)) (0.0 1.0 0.0))) false false)
  (return (`local.LocalLocation`)))

(fn `UserConstructionScript`)