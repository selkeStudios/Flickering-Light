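; Moving ledge actor that slides its Cube along X between bounds offset from its start position.
; Tick steps the position by ExtraSpeed, with delayed direction flips at the bounds, and zeroes that speed under heavy slow motion.
; A Flicker entering the Box gets StopAndFlick and halts the ledge if alive; its exit restores speed after a delay.
; Overlap with an enigMaticForce destroys the ledge.
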(event `self.ReceiveActorBeginOverlap`
  (params (OtherActor :type "Actor Object Reference"))
  (cast `/Game/Blueprints/enigmaticForce` OtherActor)
  (`/Engine/EditorBlueprintResources/StandardMacros.IsValid` (`self.Box`)
    (:`Is Valid`
      (`self.K2_DestroyActor`))))

(event `self.ReceiveBeginPlay`
  (set `self.beginningLoc` (.x (.location (`SceneComponent.GetRelativeTransform` (`self.Cube`)))))
  (set `self.leftEnd` (+ (`self.beginningLoc`) (`self.ricocheteValue`)))
  (set `self.rightEnd` (- (`self.beginningLoc`) (`self.ricocheteValue`))))

(event `self.Box.OnComponentBeginOverlap`
  (params (OverlappedComponent :type "PrimitiveComponent Object Reference") (OtherActor :type "Actor Object Reference") (OtherComp :type "PrimitiveComponent Object Reference") (OtherBodyIndex :type Integer) (bFromSweep :type Boolean) (SweepResult :type "HitResult Structure (by ref)"))
  (bind _asflicker (cast `/Game/FlickerBPs/Blueprints/Flicker` OtherActor))
  (`/Engine/EditorBlueprintResources/StandardMacros.IsValid` (`self.Box`)
    (:`Is Valid`
      (`/Game/FlickerBPs/Blueprints/Flicker.stopAndFlick` _asflicker (`self.Cube`))
      (if (not (`/Game/FlickerBPs/Blueprints/Flicker.isDead` _asflicker))
        (set `self.extraSpeed` 0.0)))))

(event `self.ReceiveTick`
  (params (DeltaSeconds :type "Float (single-precision)"))
  (bind _returnvalue (`SceneComponent.GetRelativeTransform` (`self.Cube`)))
  (bind _returnvalue_2 (`SceneComponent.GetRelativeTransform` (`self.Cube`)))
  (if (<= (`GameplayStatics.GetGlobalTimeDilation`) 0.2)
    (set `self.extraSpeed` 0.0)
    (else
      (bind _output_get (set `self.moveSpeed` (`KismetMathLibrary.SelectFloat` (+ (`self.moveSpeed`) (`self.extraSpeed`)) (- (`self.moveSpeed`) (`self.extraSpeed`)) (`self.moveLeft`)) :!label _label))
      (`SceneComponent.K2_SetRelativeLocation` (`self.Cube`) (`KismetMathLibrary.MakeVector` _output_get (.y (.location _returnvalue)) (.z (.location _returnvalue))) false false)
      (if (>= (.x (.location _returnvalue_2)) (`self.rightEnd`))
        (`KismetSystemLibrary.Delay` 1.0)
        (set `self.moveLeft` false)
        (elif (< (.x (.location _returnvalue_2)) (`self.leftEnd`))
          (`KismetSystemLibrary.Delay` 1.0)
          (set `self.moveLeft` true)
          (else
            (goto _label)))))))

(event `self.Box.OnComponentEndOverlap`
  (params (OverlappedComponent :type "PrimitiveComponent Object Reference") (OtherActor :type "Actor Object Reference") (OtherComp :type "PrimitiveComponent Object Reference") (OtherBodyIndex :type Integer))
  (cast `/Game/FlickerBPs/Blueprints/Flicker` OtherActor)
  (`/Engine/EditorBlueprintResources/StandardMacros.IsValid` (`self.Box`)
    (:`Is Valid`
      (`KismetSystemLibrary.Delay` 0.5)
      (set `self.extraSpeed` 3.0))))

(fn `moveBandF`
  (params (speed :type "Float (double-precision)"))
  (returns (movingComponent :type "StaticMeshComponent Object Reference") (newLoc :type "Vector Structure"))
  (bind _cube (`self.Cube`))
  (bind (_relativelocation_x _relativelocation_y _relativelocation_z) (`KismetMathLibrary.BreakVector` (`SceneComponent.RelativeLocation` _cube)))
  (return _cube (`KismetMathLibrary.MakeVector` (+ _relativelocation_x speed) _relativelocation_y _relativelocation_z)))

(fn `UserConstructionScript`)