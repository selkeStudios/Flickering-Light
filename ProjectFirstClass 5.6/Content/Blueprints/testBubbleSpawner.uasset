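; Test spawner actor that emits Force_bubbleParticle_BP actors at its Arrow's location while rising.
; SetParent attaches it to the EnigMaticForce actor found in the level and sets CanStart, which enables the Tick logic.
; Each tick, SpawnBubbles decrements a frame-based countdown, spawning and resetting at zero, and MoveComponentTo targets a point BubbleSpaawnUPSpeed above the root's relative location.
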(event `self.ReceiveBeginPlay`
  (set `self.countDown` (`self.startTime`)))

(event `self.ReceiveTick`
  (params (DeltaSeconds :type "Float (single-precision)"))
  (bind (_relativelocation_x _relativelocation_y _relativelocation_z) (`KismetMathLibrary.BreakVector` (`SceneComponent.RelativeLocation` (`self.DefaultSceneRoot`))))
  (if (`self.canStart`)
    (`self.spawnBubbles`)
    (`KismetSystemLibrary.MoveComponentTo` null (`KismetMathLibrary.MakeVector` _relativelocation_x _relativelocation_y (+ _relativelocation_z (`self.bubbleSpaawnUPSpeed`))))))

(fn `setParent`
  (bind _returnvalue (`GameplayStatics.GetActorOfClass` "/Game/Blueprints/enigMaticForce.enigMaticForce_C"))
  (`self.K2_AttachToActor` _returnvalue "None" "KeepRelative" "KeepRelative" "KeepRelative")
  (set `self.canStart` true))

(fn `spawnBubbles`
  (bind _countdown (`self.countDown`))
  (bind _returnvalue (`SceneComponent.K2_GetComponentToWorld` (`self.Arrow`)))
  (set `self.countDown` (- _countdown 1.0))
  (if (<= _countdown 0.0)
    (`|SpawnActorFromClass` "/Game/Blueprints/force_bubbleParticle_BP.force_bubbleParticle_BP_C" (`KismetMathLibrary.MakeTransform` (`KismetMathLibrary.MakeVector` (.x (.location _returnvalue)) (.y (.location _returnvalue)) (.z (.location _returnvalue)))) "Undefined" "OverrideRootScale" null null)
    (set `self.countDown` (`self.startTime`))))

(fn `UserConstructionScript`)