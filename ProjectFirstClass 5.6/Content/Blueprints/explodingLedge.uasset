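; Ledge actor that shrinks away while a living Flicker is inside its Box trigger.
; Box overlaps toggle CanShrink, and Tick reduces the Cube's X scale by ShrinkTime each frame, unscaled by delta time, destroying everything near zero.
; Actor overlap with a Flicker calls its StopAndFlick with the Cube, and an enigMaticForce ending overlap destroys the ledge immediately.
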(event `self.ReceiveBeginPlay`)

(event `self.ReceiveActorEndOverlap`
  (params (OtherActor :type "Actor Object Reference"))
  (cast `/Game/Blueprints/enigmaticForce` OtherActor)
  (`self.K2_DestroyActor`))

(event `self.ReceiveActorBeginOverlap`
  (params (OtherActor :type "Actor Object Reference"))
  (bind _asflicker (cast `/Game/FlickerBPs/Blueprints/Flicker` OtherActor))
  (`/Game/FlickerBPs/Blueprints/Flicker.stopAndFlick` _asflicker (`self.Cube`)))

(event `self.ReceiveTick`
  (params (DeltaSeconds :type "Float (single-precision)"))
  (bind _cube (`self.Cube`))
  (bind _returnvalue (`SceneComponent.GetRelativeTransform` _cube))
  (if (`self.canShrink`)
    (bind _output_get (set `self.cubeShrink` (- (`self.cubeShrink`) (`self.shrinkTime`))))
    (`SceneComponent.K2_SetRelativeTransform` _cube (`KismetMathLibrary.MakeTransform` (.location _returnvalue) (.rotation _returnvalue) (`KismetMathLibrary.MakeVector` _output_get (.y (.scale _returnvalue)) (.z (.scale _returnvalue)))) false false)
    (if (<= (.x (.scale _returnvalue)) 0.01)
      (set `self.hasBeenDestroyed` true)
      (`ActorComponent.K2_DestroyComponent` (`self.Cube`))
      (`ActorComponent.K2_DestroyComponent` (`self.Box`))
      (`self.K2_DestroyActor`))))

(event `self.Box.OnComponentBeginOverlap`
  (params (OverlappedComponent :type "PrimitiveComponent Object Reference") (OtherActor :type "Actor Object Reference") (OtherComp :type "PrimitiveComponent Object Reference") (OtherBodyIndex :type Integer) (bFromSweep :type Boolean) (SweepResult :type "HitResult Structure (by ref)"))
  (bind _asflicker (cast `/Game/FlickerBPs/Blueprints/Flicker` OtherActor))
  (if (not (`/Game/FlickerBPs/Blueprints/Flicker.isDead` _asflicker))
    (set `self.canShrink` true)))

(event `self.Box.OnComponentEndOverlap`
  (params (OverlappedComponent :type "PrimitiveComponent Object Reference") (OtherActor :type "Actor Object Reference") (OtherComp :type "PrimitiveComponent Object Reference") (OtherBodyIndex :type Integer))
  (cast `/Game/FlickerBPs/Blueprints/Flicker` OtherActor)
  (set `self.canShrink` false))

(fn `UserConstructionScript`)