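; Actor Blueprint for a force bubble particle: a sprite that rises, spins and shrinks until it removes itself.
; Each Tick raises the capsule component by MoveUpSpeed, subtracts ScaleSpeed from its scale and adds RotateSpeed to the sprite's pitch.
; The steps are applied per frame without delta time, so the speed depends on frame rate.
; The actor destroys itself once all three scale axes are nearly zero.
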(event `self.ReceiveBeginPlay`)

(event `self.ReceiveTick`
  (params (DeltaSeconds :type "Float (single-precision)"))
  (bind _capsulecomponent (`self.CapsuleComponent`))
  (bind _scalespeed (`self.scaleSpeed`))
  (bind _sprite (`self.Sprite`))
  (bind _returnvalue (`SceneComponent.GetRelativeTransform` _capsulecomponent))
  (bind (_relativerotation_roll _relativerotation_pitch _relativerotation_yaw) (`KismetMathLibrary.BreakRotator` (`SceneComponent.RelativeRotation` _sprite)))
  (`SceneComponent.K2_SetWorldTransform` _capsulecomponent (`KismetMathLibrary.MakeTransform` (`KismetMathLibrary.MakeVector` (.x (.location _returnvalue)) (.y (.location _returnvalue)) (+ (.z (.location _returnvalue)) (`self.moveUpSpeed`))) (.rotation _returnvalue) (`KismetMathLibrary.MakeVector` (- (.x (.scale _returnvalue)) _scalespeed) (- (.y (.scale _returnvalue)) _scalespeed) (- (.z (.scale _returnvalue)) _scalespeed))) false false)
  (`SceneComponent.K2_SetWorldRotation` _sprite (`KismetMathLibrary.MakeRotator` _relativerotation_roll (+ _relativerotation_pitch (`self.rotateSpeed`)) _relativerotation_yaw) false false)
  (if (and (<= (.x (.scale _returnvalue)) 0.01) (<= (.y (.scale _returnvalue)) 0.01) (<= (.z (.scale _returnvalue)) 0.01))
    (`self.K2_DestroyActor`)))

(fn `UserConstructionScript`)