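; Player character for a touch-controlled flick-jumping game, launched between ledges with height as the score.
; Dragging spawns prediction orbs along the projected path; release applies an impulse and a random flip animation.
; StopAndFlick freezes the character on a ledge and re-enables flicking, shown through material blend color.
; Out-of-bounds or enigMaticForce contact triggers Death: hit-stop time dilation, detached camera, spinning fall and high score save.
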(event `Key|R`
  (params (Key :type "Key Structure"))
  ;[1 1 1] DEBUG Keys (Delete when done)
)

(event `Key|D`
  (params (Key :type "Key Structure"))
  ;[1 1 1] DEBUG Keys (Delete when done)
)

(event `Key|F`
  (params (Key :type "Key Structure"))
  ;[1 1 1] DEBUG Keys (Delete when done)
)

(event `self.ReceiveBeginPlay`
  (`SkeletalMeshComponent.PlayAnimation` (`self.Mesh`) "/Game/FlickerBPs/Blueprints/backwardsSway.backwardsSway" true)
  (`self.SetEyeValue` 0.0))

(event `self.ReceiveTick`
  (params (DeltaSeconds :type "Float (single-precision)"))
  (bind _flickpowermultiplier (`self.flickPowerMultiplier`))
  (bind _capsulecomponent (`self.CapsuleComponent`))
  (bind _mesh (`self.Mesh`))
  (bind (_clickoriginalpos_x _clickoriginalpos_y) (`KismetMathLibrary.BreakVector2D` (`self.clickOriginalPos`)))
  (bind _canflick (`self.canFlick`))
  (bind (_returnvalue_x _returnvalue_y _returnvalue_z) (`KismetMathLibrary.BreakVector` (`SceneComponent.K2_GetComponentLocation` _capsulecomponent)))
  (bind (_returnvalue_roll _returnvalue_pitch _returnvalue_yaw) (`KismetMathLibrary.BreakRotator` (`SceneComponent.K2_GetComponentRotation` _mesh)))
  (bind (_returnvalue_x_2 _returnvalue_y_2 _returnvalue_z_2) (`KismetMathLibrary.BreakVector` (`SceneComponent.K2_GetComponentLocation` (`self.CapsuleComponent`))))
  (bind (_locationx _locationy) (`PlayerController.GetInputTouchState` (`GameplayStatics.GetPlayerController` 0) "Touch1"))
  (bind (_returnvalue_x_3 _returnvalue_y_3) (`KismetMathLibrary.BreakVector2D` (- (`KismetMathLibrary.MakeVector2D` _locationx _locationy) (`KismetMathLibrary.MakeVector2D` _clickoriginalpos_x _clickoriginalpos_y))))
  (bind _returnvalue (/ (- _returnvalue_z_2 178.34491) 10.0))
  (if (`self.hitStop`)
    (`GameplayStatics.SetGlobalTimeDilation` 0.2)
    (`KismetSystemLibrary.Delay` 0.13)
    (`GameplayStatics.SetGlobalTimeDilation` 1.0)
    (set `self.hitStop` false)
    (set `self.hasbeenHitStopped` true)
    (elif (`self.isDead`)
      (if (<= _returnvalue_z -1500.0)
        (`SceneComponent.K2_SetWorldLocation` _capsulecomponent (4000.0 0.0 4000.0) false false))
      (`SceneComponent.K2_SetWorldRotation` _mesh (`KismetMathLibrary.MakeRotator` (+ _returnvalue_roll (`self.deathRotatingSpeed`)) _returnvalue_pitch _returnvalue_yaw) false false)
      (elif (`self.playTheGame`)
        (if (> _returnvalue 0.0)
          (set `self.playerHeight` _returnvalue)
          (else
            (set `self.playerHeight` 0.0)))
        (if _canflick
          (`self.SetBlendColor` _canflick)
          (if (`self.shouldPredict`)
            (set `self.newClickPos` (`KismetMathLibrary.MakeVector2D` _locationx _locationy))
            (bind (_outhit _outpathpositions) (`GameplayStatics.Blueprint_PredictProjectilePath_ByTraceChannel` :`StartPos` (`SceneComponent.K2_GetComponentLocation` (`self.launchPos`)) :`LaunchVelocity` (`KismetMathLibrary.MakeVector` (* _returnvalue_x_3 _flickpowermultiplier) 0.0 (* _returnvalue_y_3 (/ _flickpowermultiplier 7.0))) :`ProjectileRadius` 3.0 :`DrawDebugTime` 5.0 :`SimFrequency` 10.0 :`MaxSimTime` 1.0 :`OverrideGravityZ` -50.0))
            (for _array_element _outpathpositions
              (bind _returnvalue_2 (`|SpawnActorFromClass` "/Game/predictionOrb.predictionOrb_C" (`KismetMathLibrary.MakeTransform` _array_element) "AlwaysSpawn" "MultiplyWithRoot" null null))
              (bind _iswithinminpower (`self.checkMinFlickPower` (`self.minPullAmt`)))
              (if _iswithinminpower
                (if (`self.canPlayPrepareSound`)
                  (`GameplayStatics.PlaySound2D` "/Game/Sound/flickerJump_Cue.flickerJump_Cue" 1.0 1.0 0.0 null null)
                  (bind _sprite (`PaperCharacter.Sprite` _returnvalue_2))
                  (`PaperFlipbookComponent.SetSpriteColor` _sprite (struct :`R` 1.0 :`G` 1.0 :`B` 1.0 :`A` 1.0))
                  (set `self.canPlayPrepareSound` false)
                  (set `self.fingerHasMoved` true))
                (else
                  (`PaperFlipbookComponent.SetSpriteColor` _sprite (struct :`R` 0.119792 :`G` 0.119792 :`B` 0.119792 :`A` 1.0))
                  (set `self.fingerHasMoved` false)))))
          (else
            (`self.SetBlendColor` _canflick)
            (if (or (or (>= _returnvalue_x_2 (`self.minXPos`)) (<= _returnvalue_x_2 (`self.maxXPos`))) (<= _returnvalue_z_2 -819.0))
              (`self.Death`)
              (elif (`self.canSpawnGlitter`)
                (if (not (`self.isDead`))
                  (`|SpawnActorFromClass` "/Game/Blueprints/glitterEffect_BP.glitterEffect_BP_C" (`SceneComponent.K2_GetComponentToWorld` (`self.glitterSpawn`)) "Undefined" "MultiplyWithRoot" null null))))))))))

(event `InputTouch`
  (params (Location :type "Vector Structure") (FingerIndex :type "ETouchIndex Enum"))
  (bind _flickpowermultiplier (`self.flickPowerMultiplier`))
  (bind _canflick (`self.canFlick`))
  (bind (_clickoriginalpos_x _clickoriginalpos_y) (`KismetMathLibrary.BreakVector2D` (`self.clickOriginalPos`)))
  (bind _minpullamt (`self.minPullAmt`))
  (bind _charactermovement (`self.CharacterMovement`))
  (bind (_newclickpos_x _newclickpos_y) (`KismetMathLibrary.BreakVector2D` (`self.newClickPos`)))
  (bind (_locationx _locationy) (`PlayerController.GetInputTouchState` (`GameplayStatics.GetPlayerController` 0) "Touch1"))
  (bind (_locationx_2 _locationy_2) (`PlayerController.GetInputTouchState` (`GameplayStatics.GetPlayerController` 0) "Touch1"))
  (bind (_returnvalue_x _returnvalue_y) (`KismetMathLibrary.BreakVector2D` (- (`KismetMathLibrary.MakeVector2D` _locationx_2 _locationy_2) (`KismetMathLibrary.MakeVector2D` _clickoriginalpos_x _clickoriginalpos_y))))
  (:`Pressed`
    (if _canflick
      (set `self.fingerHasMoved` false)
      (bind _output_get (set `self.clickOriginalPos` (`KismetMathLibrary.MakeVector2D` _locationx _locationy)))))
  (:`Released`
    (if _canflick
      (set `self.shouldPredict` false)
      (set `self.canPlayPrepareSound` true)
      (if (and (`self.playTheGame`) (`self.fingerHasMoved`))
        (set `CharacterMovementComponent.GravityScale` 0.5 _charactermovement)
        (if (`self.canSendFlickerFlying`)
          (`CharacterMovementComponent.AddImpulse` _charactermovement (`KismetMathLibrary.MakeVector` (* _returnvalue_x _flickpowermultiplier) 0.0 (* _returnvalue_y (/ _flickpowermultiplier 7.0))) true)
          (if (`self.inStartingArea`)
            (if (or (and (<= _newclickpos_y (- (`.Y` (`KismetMathLibrary.BreakVector2D` _output_get)) _minpullamt)) (>= _newclickpos_x (+ (`KismetMathLibrary.BreakVector2D` _output_get) _minpullamt)) (<= _newclickpos_x (- (`KismetMathLibrary.BreakVector2D` _output_get) _minpullamt))) (>= _newclickpos_y (+ (`.Y` (`KismetMathLibrary.BreakVector2D` _output_get)) _minpullamt)))
              (`GameplayStatics.PlaySound2D` "/Game/Sound/flickerJump3_Cue.flickerJump3_Cue" 1.0 1.0 0.0 null null :!label _label)
              (`self.FlickerFlip`))
            (else
              (set `self.canFlick` false)
              (set `self.canSpawnGlitter` true)
              (goto _label)))))))
  (:`Moved`
    (if _canflick
      (set `self.shouldPredict` true)
      (if (`self.fingerHasMoved`)
        _
        (elif (not (`self.canPlayPrepareSound`))
          (`GameplayStatics.PlaySound2D` "/Game/Sound/flickRetract_Cue.flickRetract_Cue" 1.0 1.0 0.0 null null)
          (set `self.canPlayPrepareSound` true))))))

(event `SaveGame`
  ;[1 1 1] Save Game
  (bind _returnvalue (`GameplayStatics.LoadGameFromSlot` "save1"))
  (bind _asbp_save_game (cast `/Game/Blueprints/BP_SaveGame` _returnvalue))
  (bind _highscore (`/Game/Blueprints/BP_SaveGame.highScore` _asbp_save_game))
  (if (or (> (`self.playerHeight`) _highscore) (> _highscore _highscore))
    (set `/Game/Blueprints/BP_SaveGame.highScore` (`self.playerHeight`) _asbp_save_game)
    (bind _foundwidgets (`WidgetBlueprintLibrary.GetAllWidgetsOfClass` "/Game/mainWidget.mainWidget_C"))
    (`TextBlock.SetText` (`/Game/mainWidget.highScoreText` (`|GetArrayItem` _foundwidgets)) (`KismetTextLibrary.Conv_IntToText` (`KismetMathLibrary.Round` _highscore)))
    (`GameplayStatics.SaveGameToSlot` _asbp_save_game "save1")))

(event `self.CapsuleComponent.OnComponentBeginOverlap`
  (params (OverlappedComponent :type "PrimitiveComponent Object Reference") (OtherActor :type "Actor Object Reference") (OtherComp :type "PrimitiveComponent Object Reference") (OtherBodyIndex :type Integer) (bFromSweep :type Boolean) (SweepResult :type "HitResult Structure (by ref)"))
  (cast `/Game/Blueprints/enigmaticForce` OtherActor)
  (`self.Death`))

(event `self.CapsuleComponent.OnComponentEndOverlap`
  (params (OverlappedComponent :type "PrimitiveComponent Object Reference") (OtherActor :type "Actor Object Reference") (OtherComp :type "PrimitiveComponent Object Reference") (OtherBodyIndex :type Integer))
  (bind _asexploding_ledge (cast `/Game/Blueprints/explodingLedge` OtherActor))
  (set `CharacterMovementComponent.GravityScale` 0.5 (`self.CharacterMovement`))
  (if (`/Game/Blueprints/explodingLedge.hasBeenDestroyed` _asexploding_ledge)
    (`SkeletalMeshComponent.PlayAnimation` (`self.Mesh`) "/Game/FlickerBPs/Blueprints/falling.falling" true)
    (`self.SetEyeValue` 0.0)))

(event `Load Game`
  (`KismetSystemLibrary.ExecuteConsoleCommand` "RestartLevel" null))

(event `RestartLevel`
  (`GameplayStatics.DeleteGameInSlot` "save1")
  (`KismetSystemLibrary.ExecuteConsoleCommand` "RestartLevel" null))

(fn `checkMinFlickPower`
  (params (minAmount :type "Float (double-precision)"))
  (returns (isWithinMinPower :type Boolean))
  (bind (_clickoriginalpos_x _clickoriginalpos_y) (`KismetMathLibrary.BreakVector2D` (`self.clickOriginalPos`)))
  (bind (_newclickpos_x _newclickpos_y) (`KismetMathLibrary.BreakVector2D` (`self.newClickPos`)))
  (return (or (or (>= _newclickpos_x (+ _clickoriginalpos_x minAmount)) (<= _newclickpos_x (- _clickoriginalpos_x minAmount))) (or (>= _newclickpos_y (+ _clickoriginalpos_y minAmount)) (<= _newclickpos_y (- _clickoriginalpos_y minAmount))))))

(fn `Death`
  (set `self.canFlick` false)
  (set `self.isDead` true)
  (set `self.playTheGame` false)
  (set `CharacterMovementComponent.GravityScale` 1.0 (`self.CharacterMovement`))
  (if (not (`self.hasbeenHitStopped`))
    (set `self.hitStop` true)
    (`PrimitiveComponent.SetCollisionEnabled` (`self.CapsuleComponent`) "NoCollision")
    (if (not (`self.deathSoundHasPlayed`))
      (`GameplayStatics.PlaySound2D` "/Game/Sound/flickerDeathSound_Cue.flickerDeathSound_Cue" 1.0 1.0 0.0 null null)
      (set `self.deathSoundHasPlayed` true))
    (`SceneComponent.K2_DetachFromComponent` (`self.FollowCamera`) "KeepWorld" "KeepWorld" "KeepWorld" true)
    (`self.SetBlendColor` false)
    (`SkeletalMeshComponent.PlayAnimation` (`self.Mesh`) "/Game/FlickerBPs/Blueprints/death.death" false)
    (`self.SetEyeValue` 0.0)
    ;[1 1 1] Implement towards end
    (`self.SaveGame`)))

(fn `FlickerFlip`
  (bind _mesh (`self.Mesh`))
  (bind _flipanimtoplay (`self.flipAnimToPlay`))
  (`KismetArrayLibrary.Array_Shuffle` _flipanimtoplay)
  (if (== (`|GetArrayItem` _flipanimtoplay) 0)
    (`SkeletalMeshComponent.PlayAnimation` _mesh "/Game/FlickerBPs/Blueprints/xFlip.xFlip" true)
    (else
      (`SkeletalMeshComponent.PlayAnimation` _mesh "/Game/FlickerBPs/Blueprints/zFlip.zFlip" true)))
  (`self.SetEyeValue` 1.0))

(fn `SetBlendColor`
  (params (isOn :type Boolean))
  (locals (Blend :type "Vector Structure" :default (0.0 0.0 0.0)) (NewLocalVar :type "Vector Structure" :default (0.0 0.0 0.0)))
  (bind _returnvalue (`KismetMathLibrary.MakeColor` 0.0))
  (bind _blend (`local.Blend`))
  (bind _mesh (`self.Mesh`))
  (if isOn
    (set `local.Blend` (`KismetMathLibrary.Conv_LinearColorToVector` (`KismetMathLibrary.MakeColor` 1.0 0.928439 0.375)))
    (else
      (set `local.Blend` (`KismetMathLibrary.Conv_LinearColorToVector` (* _returnvalue _returnvalue)))))
  (`MeshComponent.SetVectorParameterValueOnMaterials` _mesh "Blend Color" _blend)
  (`MeshComponent.SetVectorParameterValueOnMaterials` _mesh "Blend Color Eyes" _blend)
  (`MeshComponent.SetVectorParameterValueOnMaterials` _mesh "Blend Color Feet" _blend))

(fn `SetEyeValue`
  (params (Value :type "Float (double-precision)"))
  (`MeshComponent.SetScalarParameterValueOnMaterials` (`self.Mesh`) "EyeValue" Value))

(fn `stopAndFlick`
  (params (collidedObject :type "StaticMeshComponent Object Reference"))
  (bind _mesh (`self.Mesh`))
  (bind (_returnvalue_x _returnvalue_y _returnvalue_z) (`KismetMathLibrary.BreakVector` (`SceneComponent.K2_GetComponentLocation` (`self.CapsuleComponent`))))
  (bind _returnvalue (`SceneComponent.K2_GetComponentToWorld` (`self.CapsuleComponent`)))
  (if (not (`self.isDead`))
    (`GameplayStatics.PlaySoundAtLocation` "/Game/Sound/ledgeGrab_Cue.ledgeGrab_Cue" (`KismetMathLibrary.MakeVector` (.x (.location _returnvalue)) (.y (.location _returnvalue)) (.z (.location _returnvalue))) (.rotation _returnvalue) 1.0 1.0 0.0 "/Game/Sound/ledgeGrabAttenuation.ledgeGrabAttenuation" null null null)
    (if (>= (.z (.location (`SceneComponent.K2_GetComponentToWorld` collidedObject))) (- _returnvalue_z (`self.ledgeThreshold`)))
      (`SkeletalMeshComponent.PlayAnimation` _mesh "/Game/FlickerBPs/Blueprints/hanging.hanging" true)
      (else
        (`SkeletalMeshComponent.PlayAnimation` _mesh "/Game/FlickerBPs/Blueprints/standingOnLedge.standingOnLedge" true)))
    (set `CharacterMovementComponent.GravityScale` 0.0 (`self.CharacterMovement`))
    (`MovementComponent.StopMovementImmediately` (`self.CharacterMovement`))
    (if (not (`self.isDead`))
      (set `self.canFlick` true)
      (set `self.canSpawnGlitter` false))))

(fn `UserConstructionScript`)