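; Background tree-trunk segment actor that chains copies of itself to build scrolling scenery from three stacked sprites.
; The first instance picks one of five trunk looks and spawns four non-chaining copies at its under-spawn points, passing the look on.
; A Flicker overlap spawns the next matching segment once, and an enigMaticForce leaving the box destroys this one.
; Tick reapplies the sprite every frame, with a one-time spacing correction for the third and fourth variants.
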(event `self.ReceiveBeginPlay`
  (bind _returnvalue (`SceneComponent.K2_GetComponentToWorld` (`self.underSpawnPos2`)))
  (bind _returnvalue_2 (`SceneComponent.K2_GetComponentToWorld` (`self.underSpawnPos3`)))
  (bind _returnvalue_3 (`SceneComponent.K2_GetComponentToWorld` (`self.underSpawnPos4`)))
  (bind _returnvalue_4 (`SceneComponent.K2_GetComponentToWorld` (`self.underSpawnPos`)))
  (`SceneComponent.K2_SetWorldRotation` (`self.RenderComponent`) (struct :`Yaw` -180.0) false false)
  (if (`self.theFirstOne`)
    (bind _output_get (set `self.randomSprite` (`KismetMathLibrary.RandomIntegerInRange` 0 4)))
    (if (or (== _output_get 3) (== _output_get 2))
      (set `self.underSpawnPosSpacingValue` 55.0))
    (bind _returnvalue_5 (`|SpawnActorFromClass` "individualBKNDTrunksBP_C" (`KismetMathLibrary.MakeTransform` (`KismetMathLibrary.MakeVector` (.x (.location _returnvalue_4)) (.y (.location _returnvalue_4)) (- (.z (.location _returnvalue_4)) (`self.underSpawnPosSpacingValue`)))) "Undefined" "MultiplyWithRoot" null null))
    (set `/Game/Geometry/individualBKNDTrunksBP.randomSprite` (`self.randomSprite`) _returnvalue_5)
    (set `/Game/Geometry/individualBKNDTrunksBP.hasSpawnedNext` true _returnvalue_5)
    (bind _returnvalue_6 (`|SpawnActorFromClass` "individualBKNDTrunksBP_C" (`KismetMathLibrary.MakeTransform` (`KismetMathLibrary.MakeVector` (.x (.location _returnvalue)) (.y (.location _returnvalue)) (- (.z (.location _returnvalue)) (`self.underSpawnPosSpacingValue`)))) "Undefined" "MultiplyWithRoot" null null))
    (set `/Game/Geometry/individualBKNDTrunksBP.randomSprite` (`self.randomSprite`) _returnvalue_6)
    (set `/Game/Geometry/individualBKNDTrunksBP.hasSpawnedNext` true _returnvalue_6)
    (bind _returnvalue_7 (`|SpawnActorFromClass` "individualBKNDTrunksBP_C" (`KismetMathLibrary.MakeTransform` (`KismetMathLibrary.MakeVector` (.x (.location _returnvalue_2)) (.y (.location _returnvalue_2)) (- (.z (.location _returnvalue_2)) (`self.underSpawnPosSpacingValue`)))) "Undefined" "MultiplyWithRoot" null null))
    (set `/Game/Geometry/individualBKNDTrunksBP.randomSprite` (`self.randomSprite`) _returnvalue_7)
    (set `/Game/Geometry/individualBKNDTrunksBP.hasSpawnedNext` true _returnvalue_7)
    (bind _returnvalue_8 (`|SpawnActorFromClass` "individualBKNDTrunksBP_C" (`KismetMathLibrary.MakeTransform` (`KismetMathLibrary.MakeVector` (.x (.location _returnvalue_3)) (.y (.location _returnvalue_3)) (- (.z (.location _returnvalue_3)) (`self.underSpawnPosSpacingValue`)))) "Undefined" "MultiplyWithRoot" null null))
    (set `/Game/Geometry/individualBKNDTrunksBP.randomSprite` (`self.randomSprite`) _returnvalue_8)
    (set `/Game/Geometry/individualBKNDTrunksBP.hasSpawnedNext` true _returnvalue_8)))

(event `self.ReceiveTick`
  (params (DeltaSeconds :type "Float (single-precision)"))
  (bind _rendercomponent (`self.RenderComponent`))
  (bind _randomsprite (`self.randomSprite`))
  (bind _sprite2 (`self.sprite2`))
  (bind _sprite3 (`self.sprite3`))
  (bind (_returnvalue_x _returnvalue_y _returnvalue_z) (`KismetMathLibrary.BreakVector` (`SceneComponent.K2_GetComponentLocation` _sprite3)))
  (bind (_returnvalue_x_2 _returnvalue_y_2 _returnvalue_z_2) (`KismetMathLibrary.BreakVector` (`SceneComponent.K2_GetComponentLocation` _rendercomponent)))
  (bind (_returnvalue_x_3 _returnvalue_y_3 _returnvalue_z_3) (`KismetMathLibrary.BreakVector` (`SceneComponent.K2_GetComponentLocation` _sprite2)))
  (if (== _randomsprite 0)
    (`PaperSpriteComponent.SetSprite` _rendercomponent "/Game/Geometry/BKNDTrunk1_Sprite.BKNDTrunk1_Sprite")
    (`PaperSpriteComponent.SetSprite` _sprite2 "/Game/Geometry/BKNDTrunk1_Sprite.BKNDTrunk1_Sprite")
    (`PaperSpriteComponent.SetSprite` _sprite3 "/Game/Geometry/BKNDTrunk1_Sprite.BKNDTrunk1_Sprite")
    (set `self.testRenderCompPlace` _returnvalue_z_2 :!label _label)
    (set `self.testSprite2Place` _returnvalue_z_3)
    (set `self.testSprite3Place` _returnvalue_z)
    (elif (== _randomsprite 1)
      (`PaperSpriteComponent.SetSprite` _rendercomponent "/Game/Geometry/BKNDTrunk2_Sprite.BKNDTrunk2_Sprite")
      (`PaperSpriteComponent.SetSprite` _sprite2 "/Game/Geometry/BKNDTrunk2_Sprite.BKNDTrunk2_Sprite")
      (`PaperSpriteComponent.SetSprite` _sprite3 "/Game/Geometry/BKNDTrunk2_Sprite.BKNDTrunk2_Sprite")
      (goto _label)
      (elif (== _randomsprite 2)
        (`self.spriteMovementCalc`)
        (`PaperSpriteComponent.SetSprite` _rendercomponent "/Game/Geometry/BKNDTrunk3_Sprite.BKNDTrunk3_Sprite")
        (`PaperSpriteComponent.SetSprite` _sprite2 "/Game/Geometry/BKNDTrunk3_Sprite.BKNDTrunk3_Sprite")
        (`PaperSpriteComponent.SetSprite` _sprite3 "/Game/Geometry/BKNDTrunk3_Sprite.BKNDTrunk3_Sprite")
        (elif (== _randomsprite 3)
          (`self.spriteMovementCalc`)
          (`PaperSpriteComponent.SetSprite` _rendercomponent "/Game/Geometry/BKNDTrunk4_Sprite.BKNDTrunk4_Sprite")
          (`PaperSpriteComponent.SetSprite` _sprite2 "/Game/Geometry/BKNDTrunk4_Sprite.BKNDTrunk4_Sprite")
          (`PaperSpriteComponent.SetSprite` _sprite3 "/Game/Geometry/BKNDTrunk4_Sprite.BKNDTrunk4_Sprite")
          (else
            (`PaperSpriteComponent.SetSprite` _rendercomponent "/Game/Geometry/BKNDTrunk5_Sprite.BKNDTrunk5_Sprite")
            (`PaperSpriteComponent.SetSprite` _sprite2 "/Game/Geometry/BKNDTrunk5_Sprite.BKNDTrunk5_Sprite")
            (`PaperSpriteComponent.SetSprite` _sprite3 "/Game/Geometry/BKNDTrunk5_Sprite.BKNDTrunk5_Sprite")))))))

(event `self.Box.OnComponentBeginOverlap`
  (params (OverlappedComponent :type "PrimitiveComponent Object Reference") (OtherActor :type "Actor Object Reference") (OtherComp :type "PrimitiveComponent Object Reference") (OtherBodyIndex :type Integer) (bFromSweep :type Boolean) (SweepResult :type "HitResult Structure (by ref)"))
  (bind _returnvalue_location (`KismetMathLibrary.BreakTransform` (`SceneComponent.K2_GetComponentToWorld` (`self.nextTrunkSpawnPos`))))
  (if (not (`self.hasSpawnedNext`))
    (cast `/Game/FlickerBPs/Blueprints/Flicker` OtherActor)
    (bind _returnvalue (`|SpawnActorFromClass` "individualBKNDTrunksBP_C" (`KismetMathLibrary.MakeTransform` _returnvalue_location) "Undefined" "MultiplyWithRoot" null null))
    (set `/Game/Geometry/individualBKNDTrunksBP.randomSprite` (`self.randomSprite`) _returnvalue)
    (set `self.hasSpawnedNext` true)))

(event `self.Box.OnComponentEndOverlap`
  (params (OverlappedComponent :type "PrimitiveComponent Object Reference") (OtherActor :type "Actor Object Reference") (OtherComp :type "PrimitiveComponent Object Reference") (OtherBodyIndex :type Integer))
  (cast `/Game/Blueprints/enigmaticForce` OtherActor)
  (`self.K2_DestroyActor`))

(fn `spriteMovementCalc`
  (bind _nexttrunkspawnpos (`self.nextTrunkSpawnPos`))
  (bind _sprite2 (`self.sprite2`))
  (bind _sprite3 (`self.sprite3`))
  (bind (_returnvalue_x _returnvalue_y _returnvalue_z) (`KismetMathLibrary.BreakVector` (`SceneComponent.K2_GetComponentLocation` _sprite2)))
  (bind (_returnvalue_x_2 _returnvalue_y_2 _returnvalue_z_2) (`KismetMathLibrary.BreakVector` (`SceneComponent.K2_GetComponentLocation` _nexttrunkspawnpos)))
  (bind (_returnvalue_x_3 _returnvalue_y_3 _returnvalue_z_3) (`KismetMathLibrary.BreakVector` (`SceneComponent.K2_GetComponentLocation` _sprite3)))
  (if (not (`self.hasMovedOnce`))
    (`SceneComponent.K2_SetWorldLocation` _sprite2 (`KismetMathLibrary.MakeVector` _returnvalue_x _returnvalue_y (+ _returnvalue_z 21.0)) false false)
    (`SceneComponent.K2_SetWorldLocation` _sprite3 (`KismetMathLibrary.MakeVector` _returnvalue_x_3 _returnvalue_y_3 (+ _returnvalue_z_3 40.0)) false false)
    (`SceneComponent.K2_SetWorldLocation` _nexttrunkspawnpos (`KismetMathLibrary.MakeVector` _returnvalue_x_2 _returnvalue_y_2 (+ _returnvalue_z_2 55.0)) false false)
    (set `self.hasMovedOnce` true)))

(fn `UserConstructionScript`)